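; Player-controlled snake (hebi) pawn, moved by MoveRight/MoveUp axes, with four body sprites trailing along its past path.
; Tick pads TransformLog with InitialTransform up to FlameEnd, then records the actor transform as a ring buffer, only while moving.
; Four indices spaced a quarter buffer apart from the oldest entry position Arrow components.
; Their relative locations drive PaperGroupedSprite instances 1–4.
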(event EventTick
  (params (DeltaSeconds :type Float%20%28single-precision%29))
  (bind _arrow1 (Variables|Default|GetArrow1))
  (bind _arrow4 (Variables|Default|GetArrow4))
  (bind _arrow2 (Variables|Default|GetArrow2))
  (bind _arrow3 (Variables|Default|GetArrow3))
  ;[1 1 1] 初期設定
  (if (== (Utilities|Array|LastIndex (Variables|Default|GetTransformLog)) (Variables|Default|GetFlameEnd))
    (if (> (Math|Vector|VectorLength (Transformation|GetVelocity)) 0.0)
      (bind _result (Math|Integer|IncrementInt (Variables|Default|GetTransIndex))
        (:%20%20
          (Utilities|Array|SetArrayElem (Variables|Default|GetTransformLog) _result (Transformation|GetActorTransform))
          (Utilities|FlowControl|Sequence
            (:then_0
              ;[1 1 1] 一番後ろ
              (if (== (Variables|Default|GetTransIndex) (Variables|Default|GetFlameEnd))
                (Variables|Default|SetIDCheck_1 0)
                (else
                  (Variables|Default|SetIDCheck_1 (+ (Variables|Default|GetTransIndex) 1)))))
            (:then_1
              ;[1 1 1] 後ろから2番目
              (if (> (+ (Variables|Default|GetIDCheck_1) (/ (Variables|Default|GetFlameEnd) 4)) (Variables|Default|GetFlameEnd))
                (Variables|Default|SetIDCheck_2 (- (+ (Variables|Default|GetIDCheck_1) (/ (Variables|Default|GetFlameEnd) 4)) (+ (Variables|Default|GetFlameEnd) 1)))
                (else
                  (Variables|Default|SetIDCheck_2 (+ (Variables|Default|GetIDCheck_1) (/ (Variables|Default|GetFlameEnd) 4))))))
            (:then_2
              ;[1 1 1] 後ろから3番目
              (if (> (+ (Variables|Default|GetIDCheck_2) (/ (Variables|Default|GetFlameEnd) 4)) (Variables|Default|GetFlameEnd))
                (Variables|Default|SetIDCheck_3 (- (+ (Variables|Default|GetIDCheck_2) (/ (Variables|Default|GetFlameEnd) 4)) (+ (Variables|Default|GetFlameEnd) 1)))
                (else
                  (Variables|Default|SetIDCheck_3 (+ (Variables|Default|GetIDCheck_2) (/ (Variables|Default|GetFlameEnd) 4))))))
            (:then_3
              ;[1 1 1] 後ろから4番目
              (if (> (+ (Variables|Default|GetIDCheck_3) (/ (Variables|Default|GetFlameEnd) 4)) (Variables|Default|GetFlameEnd))
                (Variables|Default|SetIDCheck_4 (- (+ (Variables|Default|GetIDCheck_3) (/ (Variables|Default|GetFlameEnd) 4)) (+ (Variables|Default|GetFlameEnd) 1)))
                (else
                  (Variables|Default|SetIDCheck_4 (+ (Variables|Default|GetIDCheck_3) (/ (Variables|Default|GetFlameEnd) 4))))))
            (:then_4
              (for (_array_element _array_index) (Variables|Default|GetTransformLog)
                (if (== (Variables|Default|GetIDCheck_1) _array_index)
                  (Transformation|SetWorldLocation _arrow1 (.Location (Math|Transform|BreakTransform _array_element)) false false)
                  (Components|InstancedStaticMesh|UpdateInstanceTransform (Variables|Default|GetPaperGroupedSprite) 1 (Math|Transform|MakeTransform (Variables|/Script/Engine.SceneComponent|GetRelativeLocation _arrow1) (Math|Rotator|MakeRotator 9e+01 0.0 0.0) "1,1,1") false true false)
                  (elif (== (Variables|Default|GetIDCheck_2) _array_index)
                    (Transformation|SetWorldLocation _arrow2 (.Location (Math|Transform|BreakTransform _array_element)) false false)
                    (Components|InstancedStaticMesh|UpdateInstanceTransform (Variables|Default|GetPaperGroupedSprite) 2 (Math|Transform|MakeTransform (Variables|/Script/Engine.SceneComponent|GetRelativeLocation _arrow2) (Math|Rotator|MakeRotator 9e+01 0.0 0.0) "1,1,1") false true false)
                    (elif (== (Variables|Default|GetIDCheck_3) _array_index)
                      (Transformation|SetWorldLocation _arrow3 (.Location (Math|Transform|BreakTransform _array_element)) false false)
                      (Components|InstancedStaticMesh|UpdateInstanceTransform (Variables|Default|GetPaperGroupedSprite) 3 (Math|Transform|MakeTransform (Variables|/Script/Engine.SceneComponent|GetRelativeLocation _arrow3) (Math|Rotator|MakeRotator 9e+01 0.0 0.0) "1,1,1") false true false)
                      (elif (== (Variables|Default|GetIDCheck_4) _array_index)
                        (Transformation|SetWorldLocation _arrow4 (.Location (Math|Transform|BreakTransform _array_element)) false false)
                        (Components|InstancedStaticMesh|UpdateInstanceTransform (Variables|Default|GetPaperGroupedSprite) 4 (Math|Transform|MakeTransform (Variables|/Script/Engine.SceneComponent|GetRelativeLocation _arrow4) (Math|Rotator|MakeRotator 9e+01 0.0 0.0) "1,1,1") false true false))))))
              (if (>= (Variables|Default|GetTransIndex) (Variables|Default|GetFlameEnd))
                (Variables|Default|SetTransIndex -1)))))))
    (else
      (Utilities|Array|Add (Variables|Default|GetTransformLog) (Variables|Default|GetInitial_Transform)))))

(event Input|AxisEvents|InputAxisMoveRight
  (params (AxisValue :type Float%20%28single-precision%29))
  (Pawn|Input|AddMovementInput "1.000000,0.000000, 0" AxisValue false))

(event Input|AxisEvents|InputAxisMoveUp
  (params (AxisValue :type Float%20%28single-precision%29))
  (Pawn|Input|AddMovementInput "0,1.000000, 0" AxisValue false))

(fn ConstructionScript)